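; BP_Cave is a cave actor that builds itself from spline mesh sections along its spline in the Construction Script.
; Section length scales with the actor's X scale, and BuildCave places one mesh per section with clamped tangents.
; In procedural mode, ProceduralSpawn first extends the spline along -Y by random distances and a fixed height step.
; With Split on, the last section gets separate mesh settings and another BP_Cave is spawned near it.
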(fn `BuildCave`
  (bind _spline (`self.Spline`))
  (bind _sectionlength (`self.SectionLength`))
  (bind _spline_2 (`self.Spline`))
  (bind _spline_3 (`self.Spline`))
  (bind _sectionlength_2 (`self.SectionLength`))
  (bind _spline_4 (`self.Spline`))
  (bind _returnvalue (* _sectionlength -1.0))
  (bind _returnvalue_2 (`KismetMathLibrary.FFloor` (/ (`SplineComponent.GetSplineLength` (`self.Spline`)) (`self.SectionLength`))))
  (bind _returnvalue_3 (- _returnvalue_2 1))
  (bind _returnvalue_4 (* _returnvalue_2 (`self.SectionLength`)))
  (bind _returnvalue_5 (* _returnvalue_3 (`self.SectionLength`)))
  (bind _returnvalue_6 (`SplineComponent.GetLocationAtDistanceAlongSpline` _spline_3 _returnvalue_5 "Local"))
  (for _index (range (+ _returnvalue_3 1))
    (if (not (and (`self.Split`) (== _index _returnvalue_3)))
      (bind _returnvalue_7 (`AddComponent|NODE_AddSplineMeshComponent-0`))
      (`SplineMeshComponent.SetForwardAxis` _returnvalue_7 "X" true)
      (bind _returnvalue_8 (* _index (`self.SectionLength`)))
      (`SplineMeshComponent.SetSplineUpDir` _returnvalue_7 (`KismetMathLibrary.RotateAngleAxis` (`SplineComponent.GetDirectionAtDistanceAlongSpline` _spline_4 _returnvalue_8 "Local") -90.0 (0.0 1.0 0.0)) true)
      (bind _returnvalue_9 (* (+ _index 1) (`self.SectionLength`)))
      (`SplineMeshComponent.SetStartAndEnd` _returnvalue_7 (`SplineComponent.GetLocationAtDistanceAlongSpline` _spline_4 _returnvalue_8 "Local") (`KismetMathLibrary.ClampVectorSize` (`SplineComponent.GetTangentAtDistanceAlongSpline` _spline_4 _returnvalue_8 "Local") _returnvalue _sectionlength) (`SplineComponent.GetLocationAtDistanceAlongSpline` _spline _returnvalue_9 "Local") (`KismetMathLibrary.ClampVectorSize` (`SplineComponent.GetTangentAtDistanceAlongSpline` _spline _returnvalue_9 "Local") _returnvalue _sectionlength) true)))
  (if (`self.Split`)
    (bind _returnvalue_10 (`AddComponent|NODE_AddSplineMeshComponent-1`))
    (`SplineMeshComponent.SetForwardAxis` _returnvalue_10 "X" true)
    (`SplineMeshComponent.SetStartAndEnd` _returnvalue_10 _returnvalue_6 (`KismetMathLibrary.ClampVectorSize` (`SplineComponent.GetTangentAtDistanceAlongSpline` _spline_3 _returnvalue_5 "Local") 0.0 _sectionlength_2) (`SplineComponent.GetLocationAtDistanceAlongSpline` _spline_2 _returnvalue_4 "Local") (`KismetMathLibrary.ClampVectorSize` (`SplineComponent.GetTangentAtDistanceAlongSpline` _spline_2 _returnvalue_4 "Local") 0.0 _sectionlength_2) true)
    (`|SpawnActorFromClass` "BP_Cave_C" (`KismetMathLibrary.MakeTransform` (+ _returnvalue_6 (370.0 0.0 0.0))) "Undefined" "OverrideRootScale" null false null)))

(fn `ProceduralSpawn`
  (bind _spline (`self.Spline`))
  (bind _height_varience (`self.Height_Varience`))
  (bind _length_varience (`self.Length_Varience`))
  (bind _numberofpieces (`self.NumberOfPieces`))
  (bind _returnvalue (- (`self.CurrentPoint`) 1))
  (bind _returnvalue_2 (`SplineComponent.GetLocationAtSplinePoint` (`self.Spline`) _returnvalue "Local"))
  (`SplineComponent.AddPoint` _spline (make `SplinePoint` 0.0 _returnvalue_2 (`SplineComponent.GetTangentAtSplinePoint` (`self.Spline`) _returnvalue "Local") (0.0 0.0 0.0) (struct) (1.0 1.0 1.0)) true)
  (if (<= _numberofpieces 0) :!label _label
    (`self.BuildCave`)
    (else
      (`SplineComponent.AddSplinePoint` _spline (+ (`KismetMathLibrary.MakeVector` 0.0 (* (`KismetMathLibrary.RandomFloatInRange` (/ _length_varience 2.0) _length_varience) -1.0) (`KismetMathLibrary.RandomFloatInRange` _height_varience _height_varience)) _returnvalue_2) "Local" true)
      (`/Engine/EditorBlueprintResources/StandardMacros.IncrementInt` (`self.CurrentPoint`)
        (:`  `
          (`/Engine/EditorBlueprintResources/StandardMacros.DecrementInt` _numberofpieces
            (:`  `
              (goto _label))))))))

(fn `UserConstructionScript`
  (bind _returnvalue_x (`KismetMathLibrary.BreakVector` (`self.GetActorScale3D`)))
  (set `self.SectionLength` (* _returnvalue_x 200.0))
  (if (`self.Procedural`)
    (`self.ProceduralSpawn`)
    (else
      (`self.BuildCave`))))